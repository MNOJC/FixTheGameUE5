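; BP_MenuController is a menu controller Blueprint that gently swivels its Camera in response to the mouse cursor.
; Each Tick it deprojects the cursor into world space and finds the look-at rotation from the camera.
; Pitch and a sign-corrected yaw are remapped into a small angular range, with roll held at zero.
; The camera's relative rotation eases toward that result through a delta-time-scaled lerp.
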(event `self.ReceiveTick`
  (params (DeltaSeconds :type "Float (single-precision)"))
  (bind _returnvalue (`GameplayStatics.GetPlayerController` 0))
  (bind _camera (`self.Camera`))
  (bind (_locationx _locationy) (`PlayerController.GetMousePosition` _returnvalue))
  (bind (_returnvalue_roll _returnvalue_pitch _returnvalue_yaw) (`KismetMathLibrary.BreakRotator` (`KismetMathLibrary.FindLookAtRotation` (`SceneComponent.K2_GetComponentLocation` _camera) (`GameplayStatics.DeprojectScreenToWorld` _returnvalue (`KismetMathLibrary.MakeVector2D` _locationx _locationy)))))
  (`SceneComponent.K2_SetRelativeRotation` _camera (`KismetMathLibrary.RLerp` (`SceneComponent.RelativeRotation` _camera) (`KismetMathLibrary.MakeRotator` 0.0 (`KismetMathLibrary.MapRangeClamped` _returnvalue_pitch -36.0 36.0 -10.0 10.0) (`KismetMathLibrary.MapRangeClamped` (`KismetMathLibrary.SelectFloat` (* _returnvalue_yaw -1.0) _returnvalue_yaw (> _returnvalue_yaw -80.0)) -80.0 -180.0 10.0 -10.0)) (* (`GameplayStatics.GetWorldDeltaSeconds`) 0.5)) false false))

(fn `UserConstructionScript`)