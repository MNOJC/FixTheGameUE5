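; BP_Turbo is a single-use turbo pickup for the offroad car.
; On BeginPlay it caches the player's HUD_Main.
; When an OffroadCar_Pawn overlaps its Box, a DoOnce calls ResetTurbo on the HUD's turbo bar widget and turns the PointLight off.
; The DoOnce is never reset, so the pickup stays in the level but spent.
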(event `self.ReceiveBeginPlay`
  (bind _ashud_main (cast `/Game/HUD/HUD_Main` (`PlayerController.GetHUD` (`GameplayStatics.GetPlayerController` 0))))
  (set `self.As HUD Main` _ashud_main))

(event `self.Box.OnComponentBeginOverlap`
  (params (OverlappedComponent :type "PrimitiveComponent Object Reference") (OtherActor :type "Actor Object Reference") (OtherComp :type "PrimitiveComponent Object Reference") (OtherBodyIndex :type Integer) (bFromSweep :type Boolean) (SweepResult :type "HitResult Structure (by ref)"))
  (bind _asoffroad_car_pawn (cast `/Game/VehicleTemplate/Blueprints/OffroadCar/OffroadCar_Pawn` OtherActor))
  (set `self.As Offroad Car Pawn` _asoffroad_car_pawn)
  (`/Engine/EditorBlueprintResources/StandardMacros.DoOnce` false
    (:`Completed`
      (`/Game/HUD/Widgets/WBP_TurboBar.ResetTurbo` (`/Game/HUD/HUD_Main.TurboBarWidget` (`self.As HUD Main`)))
      (`LightComponent.SetIntensity` (`self.PointLight`) 0.0))))

(fn `UserConstructionScript`)